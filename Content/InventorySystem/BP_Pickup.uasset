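; World pickup actor that gives its inventory item to whoever interacts with it.
; On construction it sets its static mesh from the item definition's WorldRep fragment.
; On interaction it adds the item to the interactor's InventoryManagerCom and destroys itself, provided that component exists.
; Getter functions supply the interaction's type, timing, location above the mesh and a prompt showing item name and count.
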(event `/Game/InteractionSystem/BPI_Interactable.Interact`
  (params (Interactor :type "Actor Object Reference"))
  (bind _returnvalue (`self.GetComponentByClass` Interactor "/Game/InventorySystem/InventoryManagerCom.InventoryManagerCom_C"))
  (`/Engine/EditorBlueprintResources/StandardMacros.IsValid` _returnvalue
    (:`Is Valid`
      (`/Game/InventorySystem/InventoryManagerCom.AddItem` _returnvalue (`self.InventoryItem`))
      (`self.K2_DestroyActor`))))

(fn `GetHoldDuration`
  (returns (duration :type "Float (double-precision)"))
  (return 0.5))

(fn `GetInteractionLocation`
  (returns (Location :type "Vector Structure"))
  (return (+ (`SceneComponent.K2_GetComponentLocation` (`self.StaticMesh`)) (0.0 0.0 40.0))))

(fn `GetInteractionPrompt`
  (returns (Value :type Text))
  (bind (_inventoryitem_itemdefinition _inventoryitem_count) (break `/Game/InventorySystem/Types/S_InventoryItemInfo` (`self.InventoryItem`)))
  (return (`|FormatText` "To Pickup {ItemName} x{Count}" (defaults `Object` _inventoryitem_itemdefinition) _inventoryitem_count)))

(fn `GetInteractionType`
  (returns (Type :type "/Game/InteractionSystem/E_InteractionType Enum"))
  (return "NewEnumerator1"))

(fn `GetTapCount`
  (returns (Value :type Integer))
  (return 0))

(fn `UserConstructionScript`
  (bind _inventoryitem_itemdefinition (break `/Game/InventorySystem/Types/S_InventoryItemInfo` (`self.InventoryItem`)))
  (bind _returnvalue (`ItemDefinition.FindFragmentByClass` _inventoryitem_itemdefinition "/Script/InventorySystem.InventoryItemFragment_WorldRep"))
  (`/Engine/EditorBlueprintResources/StandardMacros.IsValid` _returnvalue
    (:`Is Valid`
      (`StaticMeshComponent.SetStaticMesh` (`self.StaticMesh`) (`InventoryItemFragment_WorldRep.ItemMesh` _returnvalue)))))
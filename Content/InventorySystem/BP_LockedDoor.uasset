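; BP_LockedDoor is an interactable door that opens when the interactor's inventory holds a lockpick with uses left.
; Interact searches the InventoryManagerCom for Item_LockPick, decrements the first usable one's LimitedUse fragment and calls OpenDoor, which blocks further interaction.
; OpenDoor plays a sound and runs a timeline lerping the door's world Z from closed to open.
; Blocked attempts or missing lockpicks play another sound; interaction getters return defaults.
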(event `OpenDoor`
  (bind _door (`self.door`))
  (bind (_returnvalue_x _returnvalue_y) (`KismetMathLibrary.BreakVector` (`SceneComponent.K2_GetComponentLocation` _door)))
  (set `self.InteractionBlocked` true)
  (`GameplayStatics.PlaySoundAtLocation` "/Engine/VREditor/Sounds/UI/Enter_Play.Enter_Play" (`self.K2_GetActorLocation`) (struct) 1.0 1.0 0.0 null null null null)
  (bind (_direction _open) (`Timeline|OpenDoorTime`)
    (:`Update`
      (`SceneComponent.K2_SetWorldLocation` _door (`KismetMathLibrary.MakeVector` _returnvalue_x _returnvalue_y (`KismetMathLibrary.Lerp` (`self.DoorClosedZ`) (`self.DoorOpenZ`) _open)) false false))))

(event `/Game/InteractionSystem/BPI_Interactable.Interact`
  (params (Interactor :type "Actor Object Reference"))
  (bind _returnvalue (`self.GetComponentByClass` Interactor "/Game/InventorySystem/InventoryManagerCom.InventoryManagerCom_C"))
  (`self.InteractionBlocked`
    (:`then`
      (`GameplayStatics.PlaySoundAtLocation` "/Engine/EditorSounds/GamePreview/EndPlayInEditor.EndPlayInEditor" (`self.K2_GetActorLocation`) (struct) 1.0 1.0 0.0 null null null null :!label _label))
    (:`else`
      (`/Engine/EditorBlueprintResources/StandardMacros.IsValid` _returnvalue
        (:`Is Valid`
          (bind _invitems (`/Game/InventorySystem/InventoryManagerCom.FindAllItems` _returnvalue "/Game/InventorySystem/Items/Item_LockPick.Item_LockPick_C"))
          (if (`KismetArrayLibrary.Array_IsNotEmpty` _invitems)
            (for _array_element _invitems
              (bind _returnvalue_2 (`ItemInstance.FindFragmentByClass` (break `/Game/InventorySystem/Types/S_InventoryItem` _array_element) "/Game/InventorySystem/Fragments/ItemFrag_LimitedUse.ItemFrag_LimitedUse_C"))
              (if (`/Game/InventorySystem/Fragments/ItemFrag_LimitedUse.HasUsesLeft` _returnvalue_2 (break `/Game/InventorySystem/Types/S_InventoryItem` _array_element))
                (`self.OpenDoor`)
                (set `self.InteractionBlocked` true)
                (`/Game/InventorySystem/Fragments/ItemFrag_LimitedUse.DecrementUsesLeft` _returnvalue_2 (break `/Game/InventorySystem/Types/S_InventoryItem` _array_element))
                (break)))
            (else
              (goto _label))))
        (:`Is Not Valid`
          (goto _label))))))

(fn `GetHoldDuration`
  (returns (duration :type "Float (double-precision)"))
  (return 0.0))

(fn `GetInteractionLocation`
  (returns (Location :type "Vector Structure"))
  (return (0.0 0.0 0.0)))

(fn `GetInteractionPrompt`
  (returns (Value :type Text))
  (return ""))

(fn `GetInteractionType`
  (returns (Type :type "/Game/InteractionSystem/E_InteractionType Enum"))
  (return "NewEnumerator0"))

(fn `GetTapCount`
  (returns (Value :type Integer))
  (return 0))

(fn `UserConstructionScript`)
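; Storage component that holds stacked item instances up to a slot limit and can transfer them to another component.
; AddItems tops up matching partial stacks through recursive FillAllEmptyStacks, then constructs ItemInstances with stats and optional rarity for new slots, returning any overflow.
; TransferItem passes an entry's definition, count, stats and rarity to the target, then removes it without checking acceptance.
; Both operations call CallStorageUpdated afterward.
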(fn `AddItems`
  (params (Item :type "/Game/InventorySystem/Types/S_InventoryItemInfo Structure"))
  (returns (Remainder :type Integer))
  (locals (Remaining :type Integer :default 0))
  (bind (_item_itemdefinition _item_count _item_statsmap _item_updatedrarity) (break `/Game/InventorySystem/Types/S_InventoryItemInfo` (`local.Item`)))
  (bind _returnvalue (`KismetMathLibrary.Min` (`/Game/InventorySystem/BFL_InventoryHelpers.GetItemMaxStackCount` _item_itemdefinition) (`local.Remaining`)))
  (bind _remainder (`self.FillAllEmptyStacks` Item_ItemDefinition_2_19D85A8B4365E5D72E53FCB0DDB0EDDF Item_Count_5_1B01934D47C638B553F0059275E128E1))
  (bind _output_get (set `local.Remaining` _remainder))
  (while (and (> _output_get 0) (< (`KismetArrayLibrary.Array_Length` (`self.InventoryItems`)) (`self.MaxStorageSize`)))
    (bind _returnvalue_2 (`|GenericCreateObject` "/Script/InventorySystem.ItemInstance"))
    (`ItemInstance.Initialzie` _returnvalue_2 _item_itemdefinition _item_statsmap)
    (if (`|EnumInequality` _item_updatedrarity)
      (`ItemInstance.SetItemRarity` _returnvalue_2 _item_updatedrarity))
    (`KismetArrayLibrary.Array_Add` (`self.InventoryItems`) (make `/Game/InventorySystem/Types/S_InventoryItem` _returnvalue_2 _returnvalue))
    (set `local.Remaining` (- (`local.Remaining`) _returnvalue)))
  (`self.StorageUpdated`)
  (return (`local.Remaining`)))

(fn `FillAllEmptyStacks`
  (params (ItemDef :type "ItemDefinition Class Reference") (TotalAmt :type Integer))
  (returns (Remainder :type Integer))
  (locals (AmtAdded :type Integer :default 0))
  (bind (_itemindex _found) (`self.FindStackWithEmptySpace` ItemDef))
  (bind _output (`|GetArrayItem` (`self.InventoryItems`) _itemindex))
  (bind (_iteminstance _count) (break `/Game/InventorySystem/Types/S_InventoryItem` _output))
  (if (<= TotalAmt 0)
    (return 0)
    (elif _found
      (bind _output_get (set `local.AmtAdded` (`KismetMathLibrary.Min` (- (`/Game/InventorySystem/BFL_InventoryHelpers.GetItemMaxStackCount` (`ItemInstance.ItemDefinition` _iteminstance)) _count) (`local.TotalAmt`))))
      (setmembers `/Game/InventorySystem/Types/S_InventoryItem` :`StructRef` _output :`Count` (+ _output_get _count))
      (bind _remainder (`self.FillAllEmptyStacks` (`local.ItemDef`) (- (`local.TotalAmt`) (`local.AmtAdded`))))
      (return _remainder)
      (else
        (return (`local.TotalAmt`))))))

(fn `FindStackWithEmptySpace`
  (params (ItemDefinition :type "ItemDefinition Class Reference"))
  (returns (ItemIndex :type Integer) (Found :type Boolean))
  (for (_array_element _array_index) (`self.InventoryItems`)
    (if (and (== (`ItemInstance.ItemDefinition` (break `/Game/InventorySystem/Types/S_InventoryItem` _array_element)) (`local.ItemDefinition`)) (< (`.Count_5_CA82A5D447607AE7124FC696C6E70DBA` (break `/Game/InventorySystem/Types/S_InventoryItem` _array_element)) (`/Game/InventorySystem/BFL_InventoryHelpers.GetItemMaxStackCount` ItemDefinition)))
      (return _array_index true)))
  (return -1 false))

(fn `TransferItem`
  (params (Index :type Integer) (Comp :type "/Game/InventorySystem/InventoryManagerCom Object Reference"))
  (bind (_output_iteminstance _output_count) (break `/Game/InventorySystem/Types/S_InventoryItem` (`|GetArrayItem` (`self.InventoryItems`) (`local.Index`))))
  (`/Game/InventorySystem/InventoryManagerCom.AddItem` Comp (make `/Game/InventorySystem/Types/S_InventoryItemInfo` (`ItemInstance.ItemDefinition` _output_iteminstance) _output_count (`ItemInstance.StatsMap` _output_iteminstance) (`ItemInstance.GetItemRarity` _output_iteminstance)))
  (`KismetArrayLibrary.Array_Remove` (`self.InventoryItems`) Index)
  (`self.StorageUpdated`))
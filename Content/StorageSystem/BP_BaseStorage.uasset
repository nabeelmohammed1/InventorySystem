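; BP_BaseStorage is a base interactable storage actor that opens an inventory UI for its storage component.
; On BeginPlay it creates a 16-slot WBP_StorageInv widget per actor and keeps it hidden in the viewport.
; Interact shows the cursor, switches player 0 to UI-only input, and opens the widget with the interactor and BPStorageComponent.
; Interaction getters supply a blank prompt, zero hold and tap values, and a point above the root.
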(event `self.ReceiveBeginPlay`
  (bind _returnvalue (`|CreateWidget` "/Game/StorageSystem/WBP_StorageInv.WBP_StorageInv_C"))
  (`UserWidget.AddToViewport` _returnvalue 0)
  (`Widget.SetVisibility` _returnvalue "Hidden")
  (set `self.StorageWidget` _returnvalue))

(event `/Game/InteractionSystem/BPI_Interactable.Interact`
  (params (Interactor :type "Actor Object Reference"))
  (bind _returnvalue (`GameplayStatics.GetPlayerController` 0))
  (bind _storagewidget (`self.StorageWidget`))
  (`UserWidget.SetOwningPlayer` _storagewidget _returnvalue)
  (set `PlayerController.bShowMouseCursor` true _returnvalue)
  (`WidgetBlueprintLibrary.SetInputMode_UIOnlyEx` _returnvalue (`self.StorageWidget`))
  (`Widget.SetVisibility` _storagewidget "Visible")
  (`/Game/StorageSystem/WBP_StorageInv.OpenWidget` _storagewidget Interactor (`self.BP_StorageComponent`)))

(fn `GetHoldDuration`
  (returns (duration :type "Float (double-precision)"))
  (return 0.0))

(fn `GetInteractionLocation`
  (returns (Location :type "Vector Structure"))
  (return (+ (`SceneComponent.K2_GetComponentLocation` (`self.DefaultSceneRoot`)) (0.0 0.0 40.0))))

(fn `GetInteractionPrompt`
  (returns (Value :type Text))
  (return ""))

(fn `GetInteractionType`
  (returns (Type :type "/Game/InteractionSystem/E_InteractionType Enum"))
  (return "NewEnumerator0"))

(fn `GetTapCount`
  (returns (Value :type Integer))
  (return 0))

(fn `UserConstructionScript`)
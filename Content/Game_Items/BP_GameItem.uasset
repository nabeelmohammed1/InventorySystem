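; Damageable game item that spawns item drops when destroyed.
; AnyDamage prints the instigator's name, subtracts damage from Health and destroys the actor once Health reaches zero or below.
; The Destroyed event loops over ItemsToDrop, spawning DropItem actors at the item's location and passing ItemType as each drop's InventoryItem.
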(event `self.ReceiveAnyDamage`
  (params (Damage :type "Float (single-precision)") (DamageType :type "DamageType Object Reference") (InstigatedBy :type "Controller Object Reference") (DamageCauser :type "Actor Object Reference"))
  (`KismetSystemLibrary.PrintString` (`KismetSystemLibrary.GetDisplayName` InstigatedBy))
  (bind _output_get (set `self.Health` (- (`self.Health`) Damage)))
  (if (<= _output_get 0.0)
    (`self.K2_DestroyActor`)))

(event `self.ReceiveDestroyed`
  (for _ (range (+ (`self.ItemsToDrop`) 1))
    (`|SpawnActorFromClass` (`self.DropItem`) (`KismetMathLibrary.MakeTransform` (`self.K2_GetActorLocation`)) "Undefined" "MultiplyWithRoot" null (`self.ItemType`) null)))

(fn `UserConstructionScript`)
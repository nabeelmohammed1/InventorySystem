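; GA_Aura_ is a Gameplay Ability child blueprint for an aura attack tied to the equipped helmet.
; On AttackStart it runs the parent logic, casts the equipped armor's spawned actor to BP_Helmet, evaluates AuraBlastTime and ends the ability.
; The branch on that result does nothing different either way, and a failed cast stops before EndAbility.
; AttackEnd is empty, and the activate and end overrides are disabled stubs.
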(event `self.Attack Start`
  (`parent.Attack Start`)
  (bind _asbp_helmet (cast `/Game/EquipmentSystem/Armor/BP_Helmet` (`EquipmentInstance.SpawnedEquipmentActor` (`self.EquippedArmor`))))
  (bind _newparam (`/Game/EquipmentSystem/Armor/BP_Helmet.AuraBlastTime` _asbp_helmet))
  (if _newparam
    _
    (else
      _))
  (`self.K2_EndAbility`))

(event `self.Attack End`)
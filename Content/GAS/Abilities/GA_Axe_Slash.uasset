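; Gameplay Ability for the axe slash, which opens and closes the equipped axe's hit scan.
; It builds on a parent ability's start and end events, casting the equipped weapon's spawned actor to BP_Axe in each.
; EventStart calls HitScan on the axe, and EventEnd calls HitScanEnd and then ends the ability.
; Activation and start also print a "Hello" debug string.
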(event `self.K2_ActivateAbility`
  (`parent.K2_ActivateAbility`)
  (`KismetSystemLibrary.PrintString` "Hello"))

(event `self.Event Start`
  (`parent.Event Start`)
  (`KismetSystemLibrary.PrintString` "Hello")
  (bind _asbp_axe (cast `/Game/EquipmentSystem/Weapons/BP_Axe` (`EquipmentInstance.SpawnedEquipmentActor` (`self.EquippedWeapon`))))
  (`/Game/EquipmentSystem/Weapons/BP_WeaponBase.HitScan` _asbp_axe))

(event `self.Event End`
  (`parent.Event End`)
  (bind _asbp_axe (cast `/Game/EquipmentSystem/Weapons/BP_Axe` (`EquipmentInstance.SpawnedEquipmentActor` (`self.EquippedWeapon`))))
  (`/Game/EquipmentSystem/Weapons/BP_WeaponBase.HitScanEnd` _asbp_axe)
  (`self.K2_EndAbility`))
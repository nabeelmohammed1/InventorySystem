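; BP_Helmet is an armor equipment actor whose only active logic is an aura blast ability.
; AuraBlastTime sweeps a large multi-sphere trace forward from the helmet on the Visibility channel, ignoring the player pawn.
; Each hit component receives an impulse along the helmet's forward vector rather than radially.
; A debug print and persistent trace drawing remain, the function always returns false, and the default events are disabled.
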(fn `AuraBlastTime`
  (returns (NewParam :type Boolean))
  (bind _returnvalue (`self.K2_GetActorLocation`))
  (`KismetSystemLibrary.PrintString` "aura")
  (bind _outhits (`KismetSystemLibrary.SphereTraceMulti` _returnvalue (+ _returnvalue (* (`self.GetActorForwardVector`) 200.0)) 500.0 "TraceTypeQuery1" false (`|MakeArray` (`GameplayStatics.GetPlayerPawn` 0) :!type "Actor Object Reference") "Persistent"))
  (for _array_element _outhits
    (`PrimitiveComponent.AddImpulse` (`.HitComponent` (`GameplayStatics.BreakHitResult` _array_element)) (* (`self.GetActorForwardVector`) 300.0) "None" false))
  (return false))

(fn `UserConstructionScript`
  (`parent.UserConstructionScript`))